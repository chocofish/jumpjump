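; Player character for a vertical jumping game that moves sideways along X, wraps at the screen edges and records its highest point reached.
; Tick updates that height and calls Die when the character drops below the camera view, which disables movement, fires OnCharacterDie and resets the height.
; Normal and double jump functions launch it upward at velocities derived from target heights via sqrt(2gh).
; IsFalling reports downward velocity, while Fly is an empty stub.
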(event EventBeginPlay)

(event Collision|EventActorBeginOverlap
  (params (OtherActor :type Actor%20Object%20Reference)))

(event EventTick
  (params (DeltaSeconds :type Float%20%28single-precision%29))
  (bind _returnvalue (Transformation|GetActorLocation))
  (bind (_x _y _z) (Math|Vector|BreakVector _returnvalue))
  ;[1 1 1] 높이 계산
  (Variables|Default|Setcharacter_height (Math|Conversions|ToFloat(Integer) (Math|Float|Ceil (Math|Float|Max(Float) (.Z (Math|Vector|BreakVector (Transformation|GetActorLocation))) (Variables|Default|Getcharacter_height)))))
  ;[1 1 1] 캐릭터가 X축 방향으로 카메라 화면을 벗어났을 경우 처리
  (if (>= _x 5.4e+02)
    (Transformation|SetActorLocation (Math|Vector|MakeVector -5.4e+02 _y _z) false false)
    (elif (<= _x -5.4e+02)
      (Transformation|SetActorLocation (Math|Vector|MakeVector 5.4e+02 _y _z) false false)))
  (if (> (- (.Z (Math|Vector|BreakVector (Transformation|GetActorLocation (Game|GetPlayerCameraManager 0)))) 9.6e+02) _z)
    (CallFunction|Die)))

(event Input|AxisEvents|InputAxisMoveRight
  (params (AxisValue :type Float%20%28single-precision%29))
  (Pawn|Input|AddMovementInput "1.000000, 0, 0" AxisValue false))

(fn ConstructionScript)

(fn JumpDouble
  (bind _velocity (CallFunction|GetVelocity (Variables|Default|Getheight_double)))
  (Character|LaunchCharacter (Math|Vector|MakeVector 0.0 0.0 _velocity) false true))

(fn JumpNormal
  (bind _velocity (CallFunction|GetVelocity (Variables|Default|Getheight_normal)))
  (Character|LaunchCharacter (Math|Vector|MakeVector 0.0 0.0 _velocity) false true))

(fn GetVelocity
  (params (height :type Float%20%28single-precision%29))
  (return (Math|Float|Power (* (* 2 9.8e+02) height) 0.5)))

(fn Die
  (Pawn|Components|CharacterMovement|SetMovementMode (Variables|Character|GetCharacterMovement) "MOVE_None" 0)
  (Default|CallCallonCharacterDie)
  (Variables|Default|Setcharacter_height 0.0))

(fn Fly)

(fn IsFalling
  (return (< (.Z (Math|Vector|BreakVector (Transformation|GetVelocity))) 0.0)))